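; BP_BaseEnemy is a base enemy Blueprint with health and reputation bar widgets and motion-warping support for facing a target.
; On BeginPlay it runs the parent logic, then sets itself as Owner on the health bar widget and, if that cast succeeds, on the reputation widget.
; UpdateFacingTarget writes a given location to the "FacingTarget" warp target on its MotionWarping component.
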(event EventBeginPlay
  (|CallParentFunction)
  (bind _aswbp_enemy_health_bar (Utilities|Casting|CastToWBP_EnemyHealthBar (UserInterface|GetUserWidgetObject (Variables|Default|GetHealthBar))))
  (Variables|/Game/UI/Enemy/WBP_EnemyHealthBar.WBP_EnemyHealthBar_C|SetOwner _aswbp_enemy_health_bar self)
  (bind _aswbp_enemy_reputation (Utilities|Casting|CastToWBP_EnemyReputation (UserInterface|GetUserWidgetObject (Variables|Default|GetReputationBar))))
  (Variables|/Game/UI/Enemy/WBP_EnemyReputation.WBP_EnemyReputation_C|SetOwner _aswbp_enemy_reputation self))

(event Collision|EventActorBeginOverlap
  (params (OtherActor :type Actor%20Object%20Reference)))

(event EventTick
  (params (DeltaSeconds :type Float%20%28single-precision%29)))

(event EventUpdateFacingTarget
  (params (Target :type Vector%20%28by%20ref%29 :default "0, 0, 0"))
  (Class|MotionWarpingComponent|AddorUpdateWarpTargetfromLocation (Variables|Default|GetMotionWarping) "FacingTarget" Target))

(fn ConstructionScript)